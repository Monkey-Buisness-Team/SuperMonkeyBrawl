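; Combat game mode for two-player monkey fights with spectator betting through Firebase.
; BeginPlay places both local players at player starts and creates a freeze-frame manager for each.
; Firebase delivers fighter profiles and scores; the fight and betting components set odds, bets open, and a 30-second Wwise-cued countdown runs.
; LaunchFight closes match bets, swaps in the fight camera and enables input; FinishCombat resets fighters and records winner and loser names.
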(event `self.ReceiveBeginPlay`
  (`parent.ReceiveBeginPlay`)
  (bind _outactors (`GameplayStatics.GetAllActorsOfClass` "/Script/Engine.PlayerStart"))
  (set `self.PlayerStartsList` _outactors)
  (bind _asch_monkey_base (cast `/Game/Characters/CH_MonkeyBase` (`GameplayStatics.GetPlayerPawn` 0)))
  (`KismetArrayLibrary.Array_Add` (`self.PlayersList`) _asch_monkey_base)
  (`self.Add Player` 1)
  (for (_array_element _array_index) (`self.PlayersList`)
    (`self.K2_SetActorLocation` _array_element (`self.K2_GetActorLocation` (`|GetArrayItem` (`self.PlayerStartsList`) (`/Game/Core/FL_SuperMonkeyBrawl.Get Other Player ID` _array_index))) false false))
  (bind _returnvalue (`|GenericCreateObject` "/Game/Core/Fight/UFreezeFrameManager.UFreezeFrameManager_C"))
  (set `self.Player1FreezeFrameManager` _returnvalue)
  (bind _returnvalue_2 (`|GenericCreateObject` "/Game/Core/Fight/UFreezeFrameManager.UFreezeFrameManager_C"))
  (set `self.Player2FreezeFrameManager` _returnvalue_2))

(event `Launch Combat Room`
  (`/Game/Firebase/FirebaseManager.OpenCloseCombatRoom` (`/Game/Core/FL_SuperMonkeyBrawl.Get Firebase Manager` (`GameplayStatics.GetGameMode`)) true)
  (add `/Game/Firebase/FirebaseManager.FighterChange` (`self.FirebaseManager`) (delegate `Fighter Received`)))

(event `Fighter Received`
  (params (data :type "/Game/Firebase/FighterData Structure") (`Is Fighter 1` :type Boolean))
  (bind _username (break `/Game/Firebase/FighterData` data))
  (bind _ac_fightmanager (`self.AC_FightManager`))
  (bind _ac_fightmanager_2 (`self.AC_FightManager`))
  (bind _firebase_manager (`/Game/Core/FL_SuperMonkeyBrawl.Get Firebase Manager` (`GameplayStatics.GetGameMode`)))
  (if (and (`KismetStringLibrary.NotEqual_StrStr` _username "Default") (`KismetStringLibrary.NotEqual_StrStr` _username))
    (`/Game/Core/Fight/AC_FightManager.Add Player Profile` (`self.AC_FightManager`) data `Is Fighter 1`)
    (if (not `Is Fighter 1`)
      (remove `/Game/Firebase/FirebaseManager.FighterChange` (`self.FirebaseManager`) (delegate `Fighter Received`))
      (`self.Retrieve Fighter Score`)
      (`KismetSystemLibrary.Delay` 1.0)
      (bind _cote (`/Game/Core/Fight/AC_FightManager.Calculate Round Player Cote` _ac_fightmanager_2 0))
      (`/Game/Core/Online/AC_ParisManager.Set Player Cote` (`self.AC_ParisManager`) 0 _cote true)
      (bind _cote_2 (`/Game/Core/Fight/AC_FightManager.Calculate Round Player Cote` _ac_fightmanager_2 0))
      (`/Game/Core/Online/AC_ParisManager.Set Player Cote` (`self.AC_ParisManager`) 0 _cote_2 false)
      (bind _cote_3 (`/Game/Core/Fight/AC_FightManager.Calculate Round Player Cote` _ac_fightmanager 1))
      (`/Game/Core/Online/AC_ParisManager.Set Player Cote` (`self.AC_ParisManager`) 1 _cote_3 true)
      (bind _cote_4 (`/Game/Core/Fight/AC_FightManager.Calculate Round Player Cote` _ac_fightmanager 1))
      (`/Game/Core/Online/AC_ParisManager.Set Player Cote` (`self.AC_ParisManager`) 1 _cote_4 false)
      (`/Game/Firebase/FirebaseManager.OpenMatchBet` _firebase_manager)
      (`/Game/Firebase/FirebaseManager.OpenRoundBet` _firebase_manager)
      (`self.StartFightLaunchTimer`)
      (`AkGameplayStatics.PostEvent` "/Game/WwiseAudio/Events/Default_Work_Unit/StartTimer.StartTimer")
      (`KismetSystemLibrary.Delay` 27.0)
      (`AkGameplayStatics.PostEvent` "/Game/WwiseAudio/Events/Default_Work_Unit/_321Fight._321Fight")
      (`KismetSystemLibrary.Delay` 3.0)
      (`self.Launch Fight`))))

(event `Retrieve Fighter Score`
  (bind _firebase_manager (`/Game/Core/FL_SuperMonkeyBrawl.Get Firebase Manager` (`GameplayStatics.GetGameMode`)))
  (add `/Game/Firebase/FirebaseManager.ScoreChange` _firebase_manager (delegate `On Score Changed`))
  (`/Game/Firebase/FirebaseManager.GetFighterScore` _firebase_manager)
  (`KismetSystemLibrary.Delay` 0.5)
  (`/Game/Firebase/FirebaseManager.GetFighterScore` _firebase_manager))

(event `On Score Changed`
  (params (Fighter1 :type "Float (double-precision)") (Fighter2 :type "Float (double-precision)"))
  (bind _playernbwin (`/Game/Core/Fight/AC_FightManager.PlayerNbWin` (`self.AC_FightManager`)))
  (`|MultiGate` false true
    (:`Out 1`
      (`BlueprintMapLibrary.Map_Add` _playernbwin 0 (`KismetMathLibrary.FTrunc` Fighter1))
      (`BlueprintMapLibrary.Map_Add` _playernbwin 1 (`KismetMathLibrary.FTrunc` Fighter2))
      (remove `/Game/Firebase/FirebaseManager.ScoreChange` (`/Game/Core/FL_SuperMonkeyBrawl.Get Firebase Manager` (`GameplayStatics.GetGameMode`)) (delegate `On Score Changed`)))))

(fn `Add Player`
  (params (ControllerId :type Integer))
  (bind _returnvalue (`GameplayStatics.GetPlayerController` ControllerId))
  (bind _playerstartslist (`self.PlayerStartsList`))
  (bind _returnvalue_2 (`KismetMathLibrary.SelectTransform` (`self.GetTransform` (`|GetArrayItem` _playerstartslist ControllerId)) (`self.GetTransform` (`|GetArrayItem` _playerstartslist)) (`KismetArrayLibrary.Array_IsValidIndex` _playerstartslist ControllerId)))
  (`/Engine/EditorBlueprintResources/StandardMacros.IsValid` (`GameplayStatics.GetPlayerController` ControllerId)
    (:`Is Valid`
      (`Controller.UnPossess` _returnvalue)
      (bind _returnvalue_3 (`|SpawnActorFromClass` "/Game/Characters/CH_MonkeyBase.CH_MonkeyBase_C" _returnvalue_2 "Undefined" "MultiplyWithRoot" null null))
      (`Controller.Possess` _returnvalue _returnvalue_3)
      (`KismetArrayLibrary.Array_Add` (`self.PlayersList`) _returnvalue_3))
    (:`Is Not Valid`
      (`KismetSystemLibrary.PrintString` "CONTROLLER DONT EXISTS")
      (bind _returnvalue_4 (`GameplayStatics.CreatePlayer` ControllerId))
      (bind _asch_monkey_base (cast `/Game/Characters/CH_MonkeyBase` (`Controller.K2_GetPawn` _returnvalue_4)))
      (`KismetArrayLibrary.Array_Add` (`self.PlayersList`) _asch_monkey_base)
      (`self.K2_SetActorTransform` _asch_monkey_base _returnvalue_2 false false))))

(fn `Finish Combat`
  (params (Winner :type Integer))
  (bind _firebase_manager (`/Game/Core/FL_SuperMonkeyBrawl.Get Firebase Manager` (`GameplayStatics.GetGameMode`)))
  (bind _playerlist (`/Game/Core/Fight/AC_FightManager.PlayerList` (`self.AC_FightManager`)))
  (bind _output_username (break `/Game/Firebase/FighterData` (`|GetArrayItem` _playerlist Winner)))
  (bind _output_username_2 (break `/Game/Firebase/FighterData` (`|GetArrayItem` _playerlist (`/Game/Core/FL_SuperMonkeyBrawl.Get Other Player ID` Winner))))
  ;[1 1 1] Todo: Ajouter UI etc
  (for _array_element (`self.PlayersList`)
    (`SceneComponent.SetVisibility` (`Character.Mesh` _array_element) false false)
    (`/Game/Characters/CH_MonkeyBase.Disable inputs` _array_element)
    (`/Game/Characters/CH_MonkeyBase.Reset Character for next round` _array_element))
  (set `/Game/Firebase/FirebaseManager.LosserName` _output_username_2 _firebase_manager)
  (`KismetSystemLibrary.PrintString` (`KismetStringLibrary.Concat_StrStr` "Winner Name" _output_username))
  (set `/Game/Firebase/FirebaseManager.WinnerName` _output_username _firebase_manager))

(fn `Init Camera`
  (bind _returnvalue (`GameplayStatics.GetActorOfClass` "/Game/Core/Fight/Camera/BP_FightCamera.BP_FightCamera_C"))
  (`/Engine/EditorBlueprintResources/StandardMacros.IsValid` _returnvalue
    (:`Is Valid`
      (`self.K2_DestroyActor` _returnvalue))
    (:`Is Not Valid`
      _))
  (bind _returnvalue_2 (`|SpawnActorFromClass` "/Game/Core/Fight/Camera/BP_FightCamera.BP_FightCamera_C" (`KismetMathLibrary.MakeTransform` (-417.0 1500.0 894.0)) "AlwaysSpawn" "MultiplyWithRoot" null null))
  (`PlayerController.SetViewTargetWithBlend` (`GameplayStatics.GetPlayerController` 0) _returnvalue_2 1.0 "VTBlend_Linear" 0.0 false)
  (`/Game/Core/Fight/Camera/BP_FightCamera.Start Camera` _returnvalue_2 (`self.PlayersList`))
  (bind _outactors (`GameplayStatics.GetAllActorsOfClass` "/Script/Engine.CameraActor"))
  (for _array_element _outactors
    (`self.K2_DestroyActor` _array_element)))

(fn `Launch Fight`
  (bind _returnvalue (`GameplayStatics.GetPlayerController` 0))
  (`/Game/Firebase/FirebaseManager.CloseMatchBet` (`/Game/Core/FL_SuperMonkeyBrawl.Get Firebase Manager` (`GameplayStatics.GetGameMode`)) false)
  (`self.Init Camera`)
  (for _array_element (`self.PlayersList`)
    (`SceneComponent.SetVisibility` (`Character.Mesh` _array_element) true false)
    (`/Game/Characters/CH_MonkeyBase.Enable inputs` _array_element))
  (`self.OnInitFightFinished`)
  (`WidgetBlueprintLibrary.SetInputMode_GameAndUIEx` _returnvalue null "DoNotLock" false)
  (set `PlayerController.bShowMouseCursor` true _returnvalue))

(fn `UserConstructionScript`)