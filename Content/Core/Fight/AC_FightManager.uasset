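; Fight manager component for the combat game mode's two-player matches, handling round flow and computing betting-style odds.
; Once fight init finishes, it listens for each player reaching zero HP, then resets characters for the next round or prints a result and reloads the level.
; Odds are inverse weighted blends of profile win rate and round wins, with round odds driven mostly by current HP.
; End-of-round and end-of-match logic are placeholders, and AddPlayerProfile stores only the first profile.
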(event Custom|On%20Init%20Fight%20Finished
  (for _array_element (Variables|/Game/Core/GM_Combat.GM_Combat_C|GetPlayersList (Variables|Default|GetGM%20Combat))
    (EventDispatchers|BindEventtoOnPlayerHPIs0 _array_element (delegate Custom|End%20Fight))))

(event Custom|End%20Fight
  (params (Player%20Number%20ID :type Integer))
  (if (== (Variables|Default|GetCurrentRound) (Variables|Default|GetNumberOfRounds))
    ;[1 1 1] Todo : à remplacer par code de fin de combat
    (Development|PrintString (Utilities|String|Append "Le joueur " (Utilities|String|ToString(Integer) (+ Player%20Number%20ID 1)) " a gagné !"))
    (bind _returnvalue (Game|GetCurrentLevelName true))
    (Game|OpenLevel(byName) (Utilities|String|StringToName _returnvalue))
    (else
      ;[1 1 1] Todo : Finir code de fin de round
      (Math|Integer|IncrementInt (Variables|Default|GetCurrentRound)
        (:%20%20
          (for _array_element (Variables|/Game/Core/GM_Combat.GM_Combat_C|GetPlayersList (Variables|Default|GetGM%20Combat))
            (Default|ResetCharacterforNextRound _array_element)))))))

(event EventBeginPlay
  (bind _asgm_combat (Utilities|Casting|CastToGM_Combat (Game|GetGameMode)))
  (bind _output_get (Variables|Default|SetGM%20Combat _asgm_combat))
  (EventDispatchers|BindEventtoOnInitFightFinished _output_get (delegate Custom|On%20Init%20Fight%20Finished)))

(fn AddPlayerProfile
  (params (Player%20Name :type Name) (Player%20ID :type String) (Player%20WinRate :type Float%20%28double-precision%29))
  (bind _playerlist (Variables|Default|GetPlayerList))
  (if (<= (Utilities|Array|Length _playerlist) 0)
    (bind _output_get (LocalVariables|SetLocale%20Player (Utilities|Struct|MakeST_PlayerProfile Player%20Name Player%20ID Player%20WinRate)))
    (Utilities|Array|Add _playerlist _output_get)
    (Default|CallOnPlayerAdded _output_get)
    (return)
    (else
      (return))))

(fn GetRoundPlayerCote
  (params (Player%20number :type Integer))
  (bind _gm_combat (Variables|Default|GetGM%20Combat))
  (bind _playernbwin (Variables|Default|GetPlayerNbWin))
  (bind _playerslist (Variables|/Game/Core/GM_Combat.GM_Combat_C|GetPlayersList _gm_combat))
  (return (|(1/(((0.025000*(((winj-winad)/2)+0.500000))+(0.900000*(((pvj-pvad)/2)+0.500000)))+(0.075000*(((vicj-vicad)/(bo+1))+0.500000)))) (Math|Conversions|ToFloat(Integer) (Utilities|Array|Get(acopy) (Variables|Default|GetPlayerNbWin) Player%20number)) (/ (Math|Conversions|ToFloat(Integer) (Default|GetHPAmount (Utilities|Array|Get(acopy) _playerslist Player%20number))) 1e+02) (Math|Conversions|ToFloat(Integer) (Variables|Default|GetNumberOfRounds)) (.playerwinrate (Utilities|Array|Get(acopy) (Variables|Default|GetPlayerList) Player%20number)) (.playerwinrate (Utilities|Array|Get(acopy) (Variables|Default|GetPlayerList) (Math|Integer|SelectInt 1 0 (== Player%20number 0)))) (/ (Math|Conversions|ToFloat(Integer) (Default|GetHPAmount (Utilities|Array|Get(acopy) _playerslist (Math|Integer|SelectInt 1 0 (== Player%20number 0))))) 1e+02) (Math|Float|SelectFloat (Math|Conversions|ToFloat(Integer) (Utilities|Array|Get(acopy) _playernbwin 1)) (Math|Conversions|ToFloat(Integer) (Utilities|Array|Get(acopy) _playernbwin)) (== Player%20number 0)))))

(fn GetMatchPlayerCote
  (params (Player%20Number :type Integer))
  (bind _returnvalue (== Player%20Number 0))
  (bind _playernbwin (Variables|Default|GetPlayerNbWin))
  (return (|(1/((0.050000*(((winj-winad)/2)+0.500000))+(0.950000*(((vicj-vicad)/(bo+1))+0.500000)))) (Math|Conversions|ToFloat(Integer) (Utilities|Array|Get(acopy) (Variables|Default|GetPlayerNbWin) Player%20Number)) (Math|Float|SelectFloat (Math|Conversions|ToFloat(Integer) (Utilities|Array|Get(acopy) _playernbwin 1)) (Math|Conversions|ToFloat(Integer) (Utilities|Array|Get(acopy) _playernbwin)) _returnvalue) (Math|Conversions|ToFloat(Integer) (Variables|Default|GetNumberOfRounds)) (.playerwinrate (Utilities|Array|Get(acopy) (Variables|Default|GetPlayerList) Player%20Number)) (.playerwinrate (Utilities|Array|Get(acopy) (Variables|Default|GetPlayerList) (Math|Integer|SelectInt 1 0 _returnvalue))))))