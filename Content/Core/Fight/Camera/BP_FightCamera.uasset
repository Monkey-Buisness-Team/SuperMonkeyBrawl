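; BP_FightCamera is a camera actor for fights that follows the first player in its list.
; StartCamera stores the players to follow and turns the camera on.
; While active, each Tick snaps BaseTransform to that player's mesh location and rotates the Camera to look at it.
; Only the first player is tracked, and movement has no smoothing.
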(event `self.ReceiveTick`
  (params (DeltaSeconds :type "Float (single-precision)"))
  (if (`self.CameraIsActive`)
    (`self.Follow Player`)))

(fn `Follow Player`
  (`SceneComponent.K2_SetWorldLocation` (`self.BaseTransform`) (`SceneComponent.K2_GetComponentLocation` (`Character.Mesh` (`|GetArrayItem` (`self.PlayersToFollow`)))) false false)
  (`SceneComponent.K2_SetWorldRotation` (`self.Camera`) (`KismetMathLibrary.FindLookAtRotation` (`SceneComponent.K2_GetComponentLocation` (`self.Camera`)) (`SceneComponent.K2_GetComponentLocation` (`self.BaseTransform`))) false false))

(fn `Start Camera`
  (params (Players :type "Array of /Game/Character/CH_MonkeyBase Object Reference"))
  (set `self.PlayersToFollow` Players)
  (set `self.CameraIsActive` true))

(fn `UserConstructionScript`)