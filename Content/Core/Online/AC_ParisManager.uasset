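; Betting manager component ("Paris" is French for bets) that tracks banana bets on two fighters, per match and per round.
; Shortly after BeginPlay it binds to the Firebase manager's bet feed, filters out placeholder names and adds each bet to that fighter's total, then fires update events.
; SetPlayerCote caches match or round odds and pushes them to Firebase.
; Resetting round totals on a new round is still a TODO.
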(event `self.ReceiveBeginPlay`
  (`KismetSystemLibrary.Delay` 0.2)
  ;[1 1 1] TODO: TotalRound a reset quand un nouveau round commence
  (add `/Game/Firebase/FirebaseManager.BetReceive` (`/Game/Core/FL_SuperMonkeyBrawl.Get Firebase Manager` (`GameplayStatics.GetGameMode`)) (`|CreateDelegate` :!event `OnBetReceive`)))

(event `OnBetReceive`
  (params (`New Bet` :type "/Game/Firebase/UserBet Structure"))
  (bind (_username _fightername _bananas _odd _ismatch) (break `/Game/Firebase/UserBet` `New Bet`))
  (bind _totalmatchbetplayer_1 (`self.TotalMatchBetPlayer_1`))
  (bind _totalroundbetplayer_1 (`self.TotalRoundBetPlayer_1`))
  (bind _totalmatchbetplayer_2 (`self.TotalMatchBetPlayer_2`))
  (bind _totalroundbetplayer_2 (`self.TotalRoundBetPlayer_2`))
  (bind _returnvalue (`KismetMathLibrary.Conv_DoubleToInt64` _bananas))
  (`KismetSystemLibrary.PrintString` _fightername)
  (`KismetSystemLibrary.PrintString` _username)
  (if (and (`KismetStringLibrary.NotEqual_StrStr` _fightername "Default") (`KismetStringLibrary.NotEqual_StrStr` _fightername) (`KismetStringLibrary.NotEqual_StrStr` _username "Default"))
    (if (== (`/Game/Core/FL_SuperMonkeyBrawl.Get Player ID By Name` (`GameplayStatics.GetGameMode`) _fightername) 0)
      (if _ismatch
        (bind _output_get (set `self.PreviousValue` (`self.TotalMatchBetPlayer_1`)))
        (`self.+=` _totalmatchbetplayer_1 _returnvalue)
        (`self.NewMatchBet` true _totalmatchbetplayer_1 _returnvalue _output_get)
        (else
          (bind _output_get_2 (set `self.PreviousValue` (`self.TotalRoundBetPlayer_1`)))
          (`self.+=` _totalroundbetplayer_1 _returnvalue)
          (`self.NewRoundBet` true _totalroundbetplayer_1 _returnvalue _output_get_2)))
      (elif _ismatch
        (bind _output_get_3 (set `self.PreviousValue` (`self.TotalMatchBetPlayer_2`)))
        (`self.+=` _totalmatchbetplayer_2 _returnvalue)
        (`self.NewMatchBet` false _totalmatchbetplayer_2 _returnvalue _output_get_3)
        (else
          (bind _output_get_4 (set `self.PreviousValue` (`self.TotalRoundBetPlayer_2`)))
          (`self.+=` _totalroundbetplayer_2 _returnvalue)
          (`self.NewRoundBet` false _totalroundbetplayer_2 _returnvalue _output_get_4))))))

(fn `+=`
  (params (VariableToModify :type "Integer64 (by ref)") (ValueToAdd :type Integer64))
  (`|VariableSetRef` VariableToModify (+ VariableToModify ValueToAdd)))

(fn `Set Player Cote`
  (params (`Player ID` :type Integer) (Cote :type "Float (double-precision)") (`isMatchCote?` :type Boolean))
  (bind _firebase_manager (`/Game/Core/FL_SuperMonkeyBrawl.Get Firebase Manager` (`GameplayStatics.GetGameMode`)))
  (bind _returnvalue (== (`local.Player ID`) 1))
  (if `isMatchCote?`
    (`BlueprintMapLibrary.Map_Add` (`self.Players Match Cotes`) `Player ID` Cote)
    (`/Game/Firebase/FirebaseManager.UpdateCoteMatch` _firebase_manager Cote _returnvalue)
    (else
      (`BlueprintMapLibrary.Map_Add` (`self.Players Round Cotes`) `Player ID` Cote)
      (`/Game/Firebase/FirebaseManager.UpdateCoteRound` _firebase_manager Cote _returnvalue))))